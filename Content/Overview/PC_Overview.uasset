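; Player controller for an overview level that pairs basic character controls with input display widgets.
; On BeginPlay it builds HUD_Overview, embeds WBP_Advanced_HUD in its RemaptDisplay slot and enables game-and-UI input.
; Any key press lazily creates an AnyKey_Overview widget once and shows the pressed key in it.
; Named inputs drive world-axis movement, jumping, and shoot/special montages that spawn projectiles from the hand socket.
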(event EventBeginPlay
  (CallFunction|CreateWidgets)
  (Input|SetInputModeGameandUI self 0 "DoNotLock" false))

(event EventTick
  (params (DeltaSeconds :type Float%20%28single-precision%29)))

(event Input|ActionEvents|InputActionJump
  (params (Key :type Key%20Structure :default "None"))
  ;[0.1063 1 0] Movement
  (:Pressed
    (bind _ascharacter (Utilities|Casting|CastToCharacter (Pawn|GetControlledPawn)))
    (Character|Jump _ascharacter)))

(event Input|ActionEvents|InputActionShoot
  (params (Key :type Key%20Structure :default "None"))
  (bind _returnvalue (Pawn|GetControlledPawn))
  (bind _ascharacter (Utilities|Casting|CastToCharacter _returnvalue))
  (bind _mesh (Variables|/Script/Engine.Character|GetMesh _ascharacter))
  (bind _returnvalue_2 (Transformation|GetSocketTransform _mesh "hand_r" "RTS_World"))
  ;[1 0.5494 0] Combat
  (:Pressed
    (Animation|Montage|PlayMontage _mesh "/Game/Overview/Animations/AM_Char_Shoot.AM_Char_Shoot"
      (:then
        (Game|SpawnActorfromClass "/Game/Overview/Projectile_Basic.Projectile_Basic_C" (Math|Transform|MakeTransform (.location _returnvalue_2) (Transformation|GetActorRotation _ascharacter) (.scale _returnvalue_2)) "AlwaysSpawn" 0 0)))))

(event Input|ActionEvents|InputActionSpecial
  (params (Key :type Key%20Structure :default "None"))
  (bind _returnvalue (Pawn|GetControlledPawn))
  (bind _ascharacter (Utilities|Casting|CastToCharacter _returnvalue))
  (bind _mesh (Variables|/Script/Engine.Character|GetMesh _ascharacter))
  (bind _returnvalue_2 (Transformation|GetSocketTransform _mesh "hand_r" "RTS_World"))
  ;[1 0.5494 0] Combat
  (:Pressed
    (Animation|Montage|PlayMontage _mesh "/Game/Overview/Animations/AM_Char_Special.AM_Char_Special"
      (:then
        (Game|SpawnActorfromClass "/Game/Overview/Projectile_Special.Projectile_Special_C" (Math|Transform|MakeTransform (.location _returnvalue_2) (Transformation|GetActorRotation _ascharacter) (.scale _returnvalue_2)) "AlwaysSpawn" 0 0)))))

(event Input|AxisEvents|InputAxisForward
  (params (AxisValue :type Float%20%28single-precision%29))
  ;[0.1063 1 0] Movement
  (Pawn|Input|AddMovementInput (Pawn|GetControlledPawn) "1.000000, 0, 0" AxisValue false))

(event Input|AxisEvents|InputAxisBackward
  (params (AxisValue :type Float%20%28single-precision%29))
  ;[0.1063 1 0] Movement
  (Pawn|Input|AddMovementInput (Pawn|GetControlledPawn) "-1.000000, 0, 0" AxisValue false))

(event Input|AxisEvents|InputAxisRight
  (params (AxisValue :type Float%20%28single-precision%29))
  ;[0.1063 1 0] Movement
  (Pawn|Input|AddMovementInput (Pawn|GetControlledPawn) "0.000000,1.000000, 0" AxisValue false))

(event Input|AxisEvents|InputAxisLeft
  (params (AxisValue :type Float%20%28single-precision%29))
  ;[0.1063 1 0] Movement
  (Pawn|Input|AddMovementInput (Pawn|GetControlledPawn) "0.000000,-1.000000, 0" AxisValue false))

(event Input|KeyboardEvents|AnyKey
  (params (Key :type Key%20Structure :default "None"))
  (:Pressed
    (Utilities|FlowControl|Sequence
      (:then_0
        (Utilities|FlowControl|DoOnce false
          (:Completed
            (bind _returnvalue (UserInterface|CreateWidget "/Game/Overview/AnyKey_Overview.AnyKey_Overview_C" self))
            (bind _output_get (Variables|Default|SetAnyKeyDisplay _returnvalue))
            (Class|ContentWidget|SetContent (Variables|/Game/Overview/HUD_Overview.HUD_Overview_C|GetKeyDisplay (Variables|Default|GetHUD)) _output_get))))
      (:then_1
        (bind _anykeydisplay (Variables|Default|GetAnyKeyDisplay)
          (:then
            (Default|ShowKey _anykeydisplay Key))
          (:else))))))

(fn ConstructionScript)

(fn CreateWidgets
  (bind _self self)
  (bind _returnvalue (UserInterface|CreateWidget "/Game/Overview/HUD_Overview.HUD_Overview_C" self))
  (Variables|Default|SetHUD _returnvalue)
  (bind _returnvalue_2 (UserInterface|CreateWidget "/Remapt/Samples/Widgets/Advanced/WBP_Advanced_HUD.WBP_Advanced_HUD_C" _self (Utilities|Struct|MakeRemaptIdentifiers _self -1 "(Name=\"\",Type=Action)" -1)))
  (Class|ContentWidget|SetContent (Variables|/Game/Overview/HUD_Overview.HUD_Overview_C|GetRemaptDisplay (Variables|Default|GetHUD)) _returnvalue_2)
  (UserInterface|Viewport|AddtoViewport (Variables|Default|GetHUD) 0))